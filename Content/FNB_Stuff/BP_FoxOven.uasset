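; BP_FoxOven is an interactable oven that bakes a bagel.
; OnInteract, an interface event, sets IsBaking, waits for BakingTimer in a Delay, then clears IsBaking and sets HasBagel.
; A branch meant to hand over a ready bagel or else start baking is disconnected, so HasBagel is never cleared here.
; Feedback is debug print strings only.
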(event EventOnInteract
  (params (player :type Character%20Object%20Reference))
  ;[1 1 1] Interface implementation: increment cooking timer, reset variables when done cooking
  (Development|PrintString "Interacted with oven")
  (Variables|Default|SetisBaking true)
  (Utilities|FlowControl|Delay (Variables|Default|GetBakingTimer))
  (Variables|Default|SetisBaking false)
  (Variables|Default|SethasBagel true)
  (Development|PrintString "Bagel Ready"))

(fn ConstructionScript)